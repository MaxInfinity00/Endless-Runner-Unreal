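; Deprecated player Blueprint for a three-lane endless runner, with lane switching, lives and death.
; Enhanced Input left/right actions offset a target position, which Tick follows with swept constant-speed interpolation.
; Capsule overlaps clear Vulnerable before the obstacle cast; obstacles cost a life and start timed invulnerability, but other overlaps leave it cleared.
; At zero lives it stops game speed, unpossesses, triggers death animation and reloads the level after a delay.
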(event `self.ReceiveBeginPlay`
  (bind _asplayer_controller (cast `PlayerController` (`self.GetController`)))
  (bind _returnvalue (pcsubsystem `EnhancedInputLocalPlayerSubsystem` _asplayer_controller))
  (`/Engine/EditorBlueprintResources/StandardMacros.IsValid` _returnvalue
    (:`Is Valid`
      (`EnhancedInputSubsystemInterface.AddMappingContext` _returnvalue "/Game/Input/RunnerInputContext.RunnerInputContext" 0 (struct))
      (set `self.DesiredPostion` (`self.K2_GetActorLocation`)))))

(event `EnhancedInput|/Game/Input/InputLeft`
  (params (ActionValue :type Boolean) (ElapsedSeconds :type "Float (double-precision)") (TriggeredSeconds :type "Float (double-precision)") (InputAction :type "InputAction Object Reference" :default "/Game/Input/InputLeft.InputLeft"))
  (:`Started`
    (if (>= (`self.Lane`) 1)
      (`/Engine/EditorBlueprintResources/StandardMacros.DecrementInt` (`self.Lane`)
        (:`  `
          (set `self.DesiredPostion` (- (`self.DesiredPostion`) (`KismetMathLibrary.MakeVector` 0.0 (`self.SwipeOffset`)))))))))

(event `EnhancedInput|/Game/Input/InputRight`
  (params (ActionValue :type Boolean) (ElapsedSeconds :type "Float (double-precision)") (TriggeredSeconds :type "Float (double-precision)") (InputAction :type "InputAction Object Reference" :default "/Game/Input/InputRight.InputRight"))
  (:`Started`
    (if (<= (`self.Lane`) 1)
      (`/Engine/EditorBlueprintResources/StandardMacros.IncrementInt` (`self.Lane`)
        (:`  `
          (set `self.DesiredPostion` (+ (`self.DesiredPostion`) (`KismetMathLibrary.MakeVector` 0.0 (`self.SwipeOffset`)))))))))

(event `self.ReceiveTick`
  (params (DeltaSeconds :type "Float (single-precision)"))
  (`self.K2_SetActorLocation` (`KismetMathLibrary.VInterpTo_Constant` (`self.K2_GetActorLocation`) (`self.DesiredPostion`) DeltaSeconds (`self.LerpStrength`)) true))

(event `self.CapsuleComponent.OnComponentBeginOverlap`
  (params (OverlappedComponent :type "PrimitiveComponent Object Reference") (OtherActor :type "Actor Object Reference") (OtherComp :type "PrimitiveComponent Object Reference") (OtherBodyIndex :type Integer) (bFromSweep :type Boolean) (SweepResult :type "HitResult Structure (by ref)"))
  (bind _lives (`self.Lives`))
  (if (`self.vulnerable`)
    (set `self.vulnerable` false)
    (cast `ObstacleComponent` OtherComp)
    (`/Engine/EditorBlueprintResources/StandardMacros.DecrementInt` _lives
      (:`  `
        (if (<= _lives 0)
          (bind _asendless_runner_game_mode_base (cast `EndlessRunnerGameModeBase` (`GameplayStatics.GetGameMode`)))
          (`EndlessRunnerGameModeBase.SetSpeed` _asendless_runner_game_mode_base 0.0)
          (`Controller.UnPossess` (`self.GetController`))
          (bind _asab_runner (cast `/Game/Runner/AB_Runner` (`SkeletalMeshComponent.GetAnimInstance` (`self.Mesh`))))
          (`/Game/Runner/AB_Runner.Die` _asab_runner)
          (`KismetSystemLibrary.Delay` 5.0)
          (`GameplayStatics.OpenLevelBySoftObjectPtr` "/Game/EndlessWorld.EndlessWorld")
          (else
            (`KismetSystemLibrary.Delay` (`self.InvulnerabilityDuration`))
            (set `self.vulnerable` true)))))))

(fn `UserConstructionScript`
  (bind _outactors (`GameplayStatics.GetAllActorsOfClass` null))
  (set `self.Ground` null))