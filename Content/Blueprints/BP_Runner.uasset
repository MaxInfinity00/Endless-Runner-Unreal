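; BP_Runner is the player-controlled runner, driving two skeletal meshes and responding to left and right swipe inputs.
; Two pairs of input actions forward to separate swipe functions, whose logic lives outside this graph.
; The Die event triggers the death animation on both meshes through their AB_Runner anim instances, then unpossesses the controller to end player control.
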(event `EnhancedInput|/Game/Input/InputLeft`
  (params (ActionValue :type Boolean) (ElapsedSeconds :type "Float (double-precision)") (TriggeredSeconds :type "Float (double-precision)") (InputAction :type "InputAction Object Reference" :default "/Game/Input/InputLeft.InputLeft"))
  (:`Started`
    (`self.SwipedLeft`)))

(event `EnhancedInput|/Game/Input/InputLeft_2`
  (params (ActionValue :type Boolean) (ElapsedSeconds :type "Float (double-precision)") (TriggeredSeconds :type "Float (double-precision)") (InputAction :type "InputAction Object Reference" :default "/Game/Input/InputLeft_2.InputLeft_2"))
  (:`Started`
    (`self.SwipedLeft2`)))

(event `EnhancedInput|/Game/Input/InputRight`
  (params (ActionValue :type Boolean) (ElapsedSeconds :type "Float (double-precision)") (TriggeredSeconds :type "Float (double-precision)") (InputAction :type "InputAction Object Reference" :default "/Game/Input/InputRight.InputRight"))
  (:`Started`
    (`self.SwipedRight`)))

(event `EnhancedInput|/Game/Input/InputRight_2`
  (params (ActionValue :type Boolean) (ElapsedSeconds :type "Float (double-precision)") (TriggeredSeconds :type "Float (double-precision)") (InputAction :type "InputAction Object Reference" :default "/Game/Input/InputRight_2.InputRight_2"))
  (:`Started`
    (`self.SwipedRight2`)))

(event `self.Die`
  (bind _asab_runner (cast `/Game/Runner/AB_Runner` (`SkeletalMeshComponent.GetAnimInstance` (`self.Mesh`))))
  (`/Game/Runner/AB_Runner.Die` _asab_runner)
  (bind _asab_runner_2 (cast `/Game/Runner/AB_Runner` (`SkeletalMeshComponent.GetAnimInstance` (`self.Mesh2`))))
  (`/Game/Runner/AB_Runner.Die` _asab_runner_2)
  (`Controller.UnPossess` (`self.GetController`)))

(fn `UserConstructionScript`)